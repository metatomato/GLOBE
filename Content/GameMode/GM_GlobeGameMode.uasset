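; GM_GlobeGameMode is a game mode that manages mode switching and spawns the UI controller on BeginPlay, exposing it through a getter.
; Registered delegates receive start, end and change messages, each followed by a matching event call.
; ChangeMode fires the change notification, which then ends the old mode and starts the new one.
; CurrentMode is updated only after those notifications are issued.
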(event EventOnGameModeStart
  (params (Mode :type GM_MODES%20Enum :default "NewEnumerator0"))
  (for _array_element (Variables|Default|GetDelegates)
    (Class|GMInterface|OnGameModeStart(Message) _array_element Mode))
  (Default|CallModeStartEvent Mode))

(event EventOnGameModeEnd
  (params (Mode :type GM_MODES%20Enum :default "NewEnumerator0"))
  (for _array_element (Variables|Default|GetDelegates)
    (Class|GMInterface|OnGameModeEnd(Message) _array_element Mode))
  (Default|CallModeEndEvent Mode))

(event EventOnGameModeChange
  (params (FromMode :type GM_MODES%20Enum :default "NewEnumerator0") (ToMode :type GM_MODES%20Enum :default "NewEnumerator0"))
  (Development|PrintString "OnGameMode Change")
  (for _array_element (Variables|Default|GetDelegates)
    (Class|GMInterface|OnGameModeChange(Message) _array_element FromMode ToMode))
  (Default|CallModeChangeEvent FromMode ToMode)
  (CallFunction|OnGameModeEnd FromMode)
  (CallFunction|OnGameModeStart ToMode))

(event EventBeginPlay
  (Development|PrintString "GAMEMODE BEGIN!")
  (bind _returnvalue (Game|SpawnActorfromClass "/Game/UI/UI_Controller.UI_Controller_C" (Variables|Default|GetDummyTransform) false 0))
  (Variables|Default|SetUIControllerInstance _returnvalue))

(fn ConstructionScript)

(fn RegisterGameModeDelegate
  (params (delegate :type GM%20Interface%20Interface))
  (Utilities|Array|Add (Variables|Default|GetDelegates) delegate))

(fn ChangeMode
  (params (Mode :type GM_MODES%20Enum :default "NewEnumerator0"))
  (CallFunction|OnGameModeChange (Variables|Default|GetCurrentMode) Mode)
  (Variables|Default|SetCurrentMode Mode))

(fn GetUIController
  (return (Variables|Default|GetUIControllerInstance)))