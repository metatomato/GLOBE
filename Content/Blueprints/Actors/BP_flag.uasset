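; BP_flag is a country flag actor that slides in and out horizontally or, as a pin flag, moves between center, surface and space positions.
; Timelines drive location lerps of the Flag component for the move-in, move-out and pull-out events.
; Construction creates a dynamic material and sets the starting position, hiding pin flags in game.
; SetTexture maps a country index to one of several 16-frame textures plus a FrameNumber parameter.
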(event Custom|MoveOutFlag
  (bind _progress (Timeline|Timeline_0 PlayFromStart)
    (:Update
      (CallFunction|MoveOut _progress))))

(event Custom|UpdateFlag
  (params (flagId :type Integer))
  (CallFunction|SetTexture flagId)
  (bind _in (Timeline|moveInTimeLine PlayFromStart)
    (:Update
      (CallFunction|Movein _in))))

(event Custom|PullOutFlag
  (params (POSITION :type Byte :default 0))
  (bind _displacement (Timeline|PullOut PlayFromStart)
    (:Update
      (switch Utilities|FlowControl|Switch|Switchon POSITION
        (:NewEnumerator0
          (CallFunction|PullFlagPin (Variables|Default|GetPinFlagCenter) "0, 0, 0" 0.0))
        (:NewEnumerator1
          (CallFunction|PullFlagPin (Variables|Default|GetPinFlagCenter) (Variables|Default|GetPinFlagSurface) _displacement))
        (:NewEnumerator2
          (CallFunction|PullFlagPin (Variables|Default|GetPinFlagCenter) (Variables|Default|GetPinFlagSpace) _displacement))))))

(fn ConstructionScript
  (bind _returnvalue (Rendering|Material|CreateDynamicMaterialInstance (Variables|Default|Getflag) 0 0 :!class /Script/Engine.PrimitiveComponent))
  (Variables|Default|SetMaterial _returnvalue)
  (Rendering|Material|SetTextureParameterValue (Variables|Default|GetMaterial) "Texture2D" "/Game/Textures/Flags/FLAG_1_1024.FLAG_1_1024")
  (if (Variables|Default|GetIsPinFlag)
    (CallFunction|PullFlagPin (Variables|Default|GetPinFlagCenter) "0, 0, 0" 0.0)
    (Development|SetHiddeninGame (Variables|Default|Getflag) true false)
    (else
      (Transformation|SetWorldLocation (Variables|Default|Getflag) (Variables|Default|GetoutLeftPosition) false))))

(fn MoveOut
  (params (achievement :type Float%20%28single-precision%29))
  (Transformation|SetWorldLocation (Variables|Default|Getflag) (Math|Vector|Lerp(Vector) (Variables|Default|GetcenterPosition) (Variables|Default|GetoutRightPosition) achievement) false))

(fn Movein
  (params (achievement :type Float%20%28single-precision%29))
  (Transformation|SetWorldLocation (Variables|Default|Getflag) (Math|Vector|Lerp(Vector) (Variables|Default|GetoutLeftPosition) (Variables|Default|GetcenterPosition) achievement) false))

(fn GetFlagIndex
  (params (coord :type Vector%202D%20Structure))
  (bind (_x _y) (Math|Vector2D|BreakVector2D coord))
  (bind _returnvalue (* _y 16.0))
  (bind _returnvalue_2 (+ _returnvalue _x))
  (Development|PrintString (Utilities|String|Append "Coord flag index " (Utilities|String|ToString(Float) _returnvalue_2)))
  (return _returnvalue_2))

(fn SetTexture
  (params (CountryIdx :type Integer))
  (bind _material (Variables|Default|GetMaterial))
  (Rendering|Material|SetTextureParameterValue _material "Texture2D" (Utilities|Array|Get(acopy) (Variables|Default|GetTextures) (/ CountryIdx 16)))
  (Rendering|Material|SetScalarParameterValue _material "FrameNumber" (Math|Conversions|ToFloat(Integer) (Math|Integer|%(Integer) CountryIdx 16)) :!class /Script/Engine.MaterialInstanceDynamic))

(fn PullFlagPin
  (params (Start :type Vector) (End :type Vector) (Progress :type Float%20%28single-precision%29))
  (Transformation|SetWorldLocation (Variables|Default|Getflag) (Math|Vector|Lerp(Vector) Start End Progress) false)
  (return))

(fn GotoSpace
  (params (Progress :type Float%20%28single-precision%29))
  (Transformation|SetWorldLocation (Variables|Default|Getflag) (Math|Vector|Lerp(Vector) (Variables|Default|GetPinFlagSurface) (Variables|Default|GetPinFlagSpace) Progress) false))