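; BP_GlobeGameMode is a game mode Blueprint that sets up the start and in-game UI.
; On BeginPlay it creates and stores both widgets, adding only the start widget to the viewport.
; RegisterGameModeDelegate collects listeners in an array, which OnModeStart iterates with an empty loop body, so no delegate is notified yet.
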(event Custom|OnModeStart
  (params (mode :type GAME_MODES%20Enum :default "NewEnumerator0"))
  (for _array_element (Variables|Default|GetGameModeDelegates)
    _))

(event EventBeginPlay
  ;[1 1 1] Init UIs
  (bind _returnvalue (UserInterface|CreateWidget "/Game/UI/UI_Start.UI_Start_C"))
  (Variables|Default|SetUIStartInstatnce _returnvalue)
  (bind _returnvalue_2 (UserInterface|CreateWidget "/Game/UI/UI_InGame.UI_InGame_C"))
  (Variables|Default|SetUIInGameInstance _returnvalue_2)
  ;[1 1 1] Create UI
  (UserInterface|Viewport|AddtoViewport (Variables|Default|GetUIStartInstatnce)))

(fn ConstructionScript)

(fn RegisterGameModeDelegate
  (params (delegate :type Game%20Mode%20Interface%20Interface))
  (Utilities|Array|Add (Variables|Default|GetGameModeDelegates) delegate))