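; Interactive globe actor that spins, rotates to given spherical coordinates and highlights countries.
; Timelines drive rotator lerps between places and slide the globe between world origin and an upper position, while Tick applies optional yaw spin.
; Clicks, touches or two-letter codes from component names toggle visibility of child country meshes, hidden at construction.
; Highlighting rescales the globe from the country's larger X or Z bound.
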(event Custom|nextPlace
  (params (location :type Vector%202D%20Structure))
  (bind _time (Timeline|Timeline_0 PlayFromStart)
    (:Update
      (CallFunction|Goto location _time))
    (:Finished
      (bind _rotator (CallFunction|ToRotator location))
      (Variables|Default|SetcurrentRotation _rotator))))

(event Custom|HighlightOffCountry
  (Rendering|SetVisibility (Variables|Country|GetCurrentHighlightedCountry) false false))

(event Custom|HighlightConutryByCode
  (params (Code :type String))
  (CallFunction|HighlightCountry (CallFunction|GetMeshfromCode Code)))

(event Custom|Highlight%20Country
  (params (StaticMesh :type Static%20Mesh%20Component%20Object%20Reference))
  (bind _code (CallFunction|GetCodefromMesh StaticMesh))
  (Development|PrintString _code)
  (Rendering|SetVisibility (Variables|Country|GetCurrentHighlightedCountry) false false)
  (if (== (Variables|Country|GetCurrentHighlightedCountry) StaticMesh)
    (Variables|Country|SetCurrentHighlightedCountry 0)
    (else
      (Variables|Country|SetCurrentHighlightedCountry StaticMesh)
      (Rendering|SetVisibility (Variables|Country|GetCurrentHighlightedCountry) true false)))
  (CallFunction|ScaleandMove (Variables|Country|GetCurrentHighlightedCountry)))

(event Custom|ScaleAndMove
  (params (Mesh :type Static%20Mesh%20Component%20Object%20Reference))
  (bind _factor (CallFunction|GetScalingFactor Mesh))
  (Transformation|SetWorldScale3D (Variables|Scene|GetScene) (Math|Vector|MakeVector _factor _factor _factor)))

(event Custom|Move
  (params (Center :type Boolean))
  (bind _upperpos (Variables|Default|GetUpperPos))
  (bind _time (Timeline|Timeline_1 PlayFromStart)
    (:Update
      (if Center
        (CallFunction|Moveto "0, 0, 0" _time)
        (else
          (CallFunction|Moveto _upperpos _time))))
    (:Finished
      (if Center
        (Variables|Default|SetcurrentPosition "0, 0, 0")
        (else
          (Variables|Default|SetcurrentPosition _upperpos))))))

(event EventTick
  (params (DeltaSeconds :type Float%20%28single-precision%29))
  (if (Variables|Default|GetisRotating)
    (Transformation|AddLocalRotation (Variables|Scene|GetScene) (Class|KismetMathLibrary|MakeRot 0.0 (* DeltaSeconds (Variables|Default|GetrotationSpeed)) 0.0) false)))

(event EventActorOnInputTouchBegin
  (params (FingerIndex :type ETouchIndex%20Enum :default "Touch1"))
  (bind _returnvalue (Game|GetPlayerController 0))
  (bind _hitresult (Game|Player|GetHitResultUnderCursorbyChannel _returnvalue "TraceTypeQuery1" true))
  (bind _hitcomponent (Collision|BreakHitResult _hitresult))
  (if (!= _hitcomponent 0)
    (bind _asstatic_mesh_component (Utilities|Casting|CastToStaticMeshComponent _hitcomponent))
    (CallFunction|HighlightCountry _asstatic_mesh_component)))

(event EventActorOnClicked
  (bind _returnvalue (Game|GetPlayerController 0))
  (bind _hitresult (Game|Player|GetHitResultUnderCursorbyChannel _returnvalue "TraceTypeQuery1" true))
  (bind _hitcomponent (Collision|BreakHitResult _hitresult))
  (if (!= _hitcomponent 0)
    (bind _asstatic_mesh_component (Utilities|Casting|CastToStaticMeshComponent _hitcomponent))
    (CallFunction|HighlightCountry _asstatic_mesh_component)))

(fn ConstructionScript
  (Transformation|SetWorldLocation (Variables|Scene|GetScene) (Variables|Default|GetcurrentPosition) false)
  (for _array_element (CallFunction|GetCountries)
    (Rendering|SetVisibility _array_element false false))
  (CallFunction|Goto (Variables|Default|GetGeoPt_RU) 1.0))

(fn SetSphericalCoord
  (params (sphericalCoords :type Vector%202D%20Structure))
  (bind _rotator (CallFunction|ToRotator sphericalCoords))
  (Transformation|SetWorldRotation (Variables|Scene|GetScene) _rotator false)
  (Variables|Default|SetcurrentRotation _rotator))

(fn SetRotating
  (params (rotationState :type Boolean))
  (Variables|Default|SetisRotating rotationState))

(fn GetRotating
  (return (Variables|Default|GetisRotating)))

(fn ToggleRotating
  (if (Variables|Default|GetisRotating)
    (Variables|Default|SetisRotating false)
    (else
      (Variables|Default|SetisRotating true))))

(fn ResetRotation
  (Transformation|SetWorldRotation (Variables|Scene|GetScene) "0, 0, 0" false))

(fn Goto
  (params (SphericalCoords :type Vector%202D%20Structure) (achievement :type Float%20%28single-precision%29))
  (bind _rotator (CallFunction|ToRotator SphericalCoords))
  (Transformation|SetWorldRotation (Variables|Scene|GetScene) (Math|Rotator|Lerp(Rotator) (Variables|Default|GetcurrentRotation) _rotator achievement) false))

(fn ToRotator
  (params (sphericalCoord :type Vector%202D%20Structure))
  (bind (_x _y) (Math|Vector2D|BreakVector2D sphericalCoord))
  (return (Math|Rotator|CombineRotators (Class|KismetMathLibrary|MakeRot 0.0 _y 0.0) (Class|KismetMathLibrary|MakeRot 0.0 0.0 _x))))

(fn Moveto
  (params (Position :type Vector) (Progress :type Float%20%28single-precision%29))
  (Transformation|SetWorldLocation (Variables|Scene|GetScene) (Math|Vector|Lerp(Vector) (Variables|Default|GetcurrentPosition) Position Progress) false))

(fn IsCountryValid
  (params (String :type String))
  (LocalVariables|Setfound false)
  (for _array_element (Variables|Country|Getcountries)
    (if (Utilities|Enum|Equal(Enum) (Utilities|Array|Get(acopy) (Utilities|String|ParseIntoArray (Utilities|GetDisplayName _array_element) " ") 1) String)
      (LocalVariables|Setfound true)))
  (return (LocalVariables|Getfound)))

(fn GetCodefromMesh
  (params (Mesh :type Static%20Mesh%20Component%20Object%20Reference))
  (bind _returnvalue (Utilities|GetDisplayName Mesh))
  (bind _returnvalue_2 (Utilities|String|Len _returnvalue))
  (return (Utilities|String|GetSubstring _returnvalue (- _returnvalue_2 2) (- _returnvalue_2 1))))

(fn GetCountries
  (for _index (range 0 (- (Class|SceneComponent|GetNumChildrenComponents (Variables|Scene|GetScene)) 1))
    (bind _asstatic_mesh_component (Utilities|Casting|CastToStaticMeshComponent (Components|GetChildComponent (Variables|Scene|GetScene) _index)))
    (Utilities|Array|Add (LocalVariables|GetLocalCountries) _asstatic_mesh_component))
  (return (LocalVariables|GetLocalCountries)))

(fn GetMeshfromCode
  (params (Country%20Code :type String))
  (for _array_element (CallFunction|GetCountries)
    (bind _code (CallFunction|GetCodefromMesh _array_element))
    (if (Utilities|Enum|Equal(Enum) _code Country%20Code)
      (return _array_element))))

(fn GenerateBox
  (params (Origin :type Vector) (Extends :type Vector))
  (bind _returnvalue (* Extends "-1.000000,1.000000,1.000000"))
  (bind _returnvalue_2 (+ Origin Extends))
  (bind _returnvalue_3 (* Extends "1.000000,1.000000,-1.000000"))
  (bind _returnvalue_4 (* Extends "-1.000000,1.000000,-1.000000"))
  (bind (_x _y _z) (Math|Vector|BreakVector _returnvalue_2))
  (bind _returnvalue_5 (+ Origin _returnvalue))
  (bind _returnvalue_6 (+ Origin _returnvalue_3))
  (bind _returnvalue_7 (+ Origin _returnvalue_4))
  (bind (_x_2 _y_2 _z_2) (Math|Vector|BreakVector _returnvalue_5))
  (bind _returnvalue_8 (Math|Vector2D|MakeVector2D _x _z))
  (bind (_x_3 _y_3 _z_3) (Math|Vector|BreakVector _returnvalue_6))
  (bind (_x_4 _y_4 _z_4) (Math|Vector|BreakVector _returnvalue_7))
  (bind _returnvalue_9 (Math|Vector2D|MakeVector2D _x_2 _z_2))
  (bind _returnvalue_10 (Math|Vector2D|MakeVector2D _x_3 _z_3))
  (bind _returnvalue_11 (Math|Vector2D|MakeVector2D _x_4 _z_4))
  (Utilities|Array|Add (LocalVariables|GetExtrema) _returnvalue_8)
  (Development|PrintString "BOX")
  (Development|PrintString (Utilities|String|ToString(Vector2d) _returnvalue_8))
  (Utilities|Array|Add (LocalVariables|GetExtrema) _returnvalue_10)
  (Development|PrintString (Utilities|String|ToString(Vector2d) _returnvalue_10))
  (Utilities|Array|Add (LocalVariables|GetExtrema) _returnvalue_11)
  (Development|PrintString (Utilities|String|ToString(Vector2d) _returnvalue_11))
  (Utilities|Array|Add (LocalVariables|GetExtrema) _returnvalue_9)
  (Development|PrintString (Utilities|String|ToString(Vector2d) _returnvalue_9))
  (return (LocalVariables|GetExtrema)))

(fn GetScalingFactor
  (params (Mesh :type Static%20Mesh%20Component%20Object%20Reference))
  (bind _boxextent (Collision|GetComponentBounds Mesh))
  (bind (_x _y _z) (Math|Vector|BreakVector _boxextent))
  (Transformation|SetWorldScale3D (Variables|Scene|GetScene) "1.000000,1.000000,1.000000")
  (Development|PrintString (Utilities|String|ToString(Vector) _boxextent))
  (if (> _x _z)
    (LocalVariables|SetScalingFactorLocal (/ (Variables|Default|GetScalingConstant) _x))
    (else
      (LocalVariables|SetScalingFactorLocal (/ (Variables|Default|GetScalingConstant) _z))))
  (Development|PrintString (Utilities|String|ToString(Float) (LocalVariables|GetScalingFactorLocal)))
  (return (LocalVariables|GetScalingFactorLocal)))