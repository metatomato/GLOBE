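; BP_pin is an actor that animates a pin between a space position and a surface position.
; PlacePin plays one timeline per direction, each feeding SetPinPosition, which lerps the actor location.
; The construction script starts the pin at SpacePos.
; Shortly after BeginPlay, InitPositions computes the surface height from the viewport's portrait aspect ratio, scaled between phone and tablet values.
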(event Custom|PlacePin
  (params (Position :type POSITIONS%20Enum :default "NewEnumerator0"))
  (switch Utilities|FlowControl|Switch|SwitchonPOSITIONS Position
    (:NewEnumerator1
      (bind _progress (Timeline|Timeline_FromSpace PlayFromStart)
        (:Update
          (CallFunction|SetPinPosition (Variables|Default|GetSpacePos) (Variables|Default|GetSurfacePos) _progress))))
    (:NewEnumerator2
      (bind _displacement (Timeline|Timeline_0 PlayFromStart)
        (:Update
          (CallFunction|SetPinPosition (Variables|Default|GetSurfacePos) (Variables|Default|GetSpacePos) _displacement))))))

(event EventBeginPlay
  (Utilities|FlowControl|Delay 0.2)
  (CallFunction|InitPositions))

(fn ConstructionScript
  (CallFunction|SetPinPosition (Variables|Default|GetSpacePos) "0, 0, 0" 0.0))

(fn SetPinPosition
  (params (Start :type Vector) (End :type Vector) (Progress :type Float%20%28single-precision%29))
  (Transformation|SetActorLocation (Math|Vector|Lerp(Vector) Start End Progress) false)
  (return))

(fn GotoSpace
  (params (Progress :type Float%20%28single-precision%29))
  (CallFunction|SetPinPosition (Variables|Default|GetSurfacePos) (Variables|Default|GetSpacePos) Progress))

(fn InitPositions
  (bind _returnvalue (Game|GetPlayerController 0))
  (bind (_sizex _sizey) (HUD|GetViewportSize _returnvalue))
  (Variables|Default|SetSurfacePos (Math|Vector|MakeVector 0.0 1e+02 (Class|MobileToolkit|ScaleValuetoScreenRatio (Math|Conversions|ToFloat(Integer) _sizex) (Math|Conversions|ToFloat(Integer) _sizey) (Variables|Default|GetPosPhone) (Variables|Default|GetPosTablet) true))))