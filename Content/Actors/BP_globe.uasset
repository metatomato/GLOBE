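; Interactive globe actor that spins, turns to given spherical coordinates and slides between the origin and an upper position.
; Timelines drive the rotation and position lerps from stored current values.
; Country meshes, gathered at construction, share one dynamic material; highlighting finds a mesh by parsed display name and fades that material's alpha.
; Click and touch handlers only print debug text or recolor the material on release; cursor-based highlighting is unwired.
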(event Custom|nextPlace
  (params (location :type Vector%202D%20Structure))
  (bind _time (Timeline|Timeline_0 PlayFromStart)
    (:Update
      (CallFunction|Goto location _time))
    (:Finished
      (bind _rotator (CallFunction|ToRotator location))
      (Variables|Default|SetcurrentRotation _rotator))))

(event Custom|Highlight%20COuntry
  (params (Name :type String) (On/Off :type Boolean))
  (bind _countrycolor (Variables|Country|GetCountryColor))
  (bind (_r _g _b) (Utilities|Struct|BreakLinearColor _countrycolor))
  (bind _exits (CallFunction|IsCountryValid Name))
  (if _exits
    (bind _countrymesh (CallFunction|GetCountryMesh Name))
    (if On/Off
      (Rendering|SetVisibility _countrymesh true false)
      (bind _alpha (Timeline|CountryMatAlpha PlayFromStart)
        (:Update
          (Rendering|Material|SetVectorParameterValue (Variables|Country|GetCountryMat) "SolidColor" (Utilities|Struct|MakeLinearColor _r _g _b _alpha) :!class /Script/Engine.MaterialInstanceDynamic))
        (:Finished
          (if (not On/Off)
            (Rendering|SetVisibility _countrymesh false false))))
      (else
        (Timeline|CountryMatAlpha ReverseFromEnd)))
    (else
      (Development|PrintString "Country Not Found!!"))))

(event Custom|Move
  (params (Center :type Boolean))
  (bind _upperpos (Variables|Default|GetUpperPos))
  (bind _time (Timeline|Timeline_1 PlayFromStart)
    (:Update
      (if Center
        (CallFunction|Moveto "0, 0, 0" _time)
        (else
          (CallFunction|Moveto _upperpos _time))))
    (:Finished
      (if Center
        (Variables|Default|SetcurrentPosition "0, 0, 0")
        (else
          (Variables|Default|SetcurrentPosition _upperpos))))))

(event EventTick
  (params (DeltaSeconds :type Float%20%28single-precision%29))
  (if (Variables|Default|GetisRotating)
    (Transformation|AddLocalRotation (Variables|Default|Getglobe) (Class|KismetMathLibrary|MakeRot 0.0 (* DeltaSeconds (Variables|Default|GetrotationSpeed)) 0.0) false)))

(event EventBeginPlay
  (Development|PrintString "GLOBE BEGIN PLAY"))

(event EventActorOnInputTouchBegin
  (params (FingerIndex :type ETouchIndex%20Enum :default "Touch1"))
  (Development|PrintString "YOU GOT ME! AAAAAAAAAAH... (silence)")
  (if (!= (.HitComponent (Collision|BreakHitResult (.HitResult (Game|Player|GetHitResultUnderCursorbyChannel (Game|GetPlayerController 0) "TraceTypeQuery1" true)))) (Variables|Default|Getglobe))
    _))

(event EventActorOnClicked
  (Development|PrintString "YOU GOT ME! AAAAAAAAAAH... (silence)")
  (if (!= (.HitComponent (Collision|BreakHitResult (.HitResult (Game|Player|GetHitResultUnderCursorbyChannel (Game|GetPlayerController 0) "TraceTypeQuery1" true)))) (Variables|Default|Getglobe))
    _))

(event EventActorOnInputTouchEnd
  (params (FingerIndex :type ETouchIndex%20Enum :default "Touch1"))
  (Rendering|Material|SetVectorParameterValue (Variables|Country|GetCountryMat) "SolidColor" "(R=0.000000,G=0.845000,B=1.000000,A=1.000000)" :!class /Script/Engine.MaterialInstanceDynamic))

(event EventActorOnReleased
  (Rendering|Material|SetVectorParameterValue (Variables|Country|GetCountryMat) "SolidColor" "(R=0.000000,G=0.845000,B=1.000000,A=1.000000)" :!class /Script/Engine.MaterialInstanceDynamic))

(fn ConstructionScript
  (bind _countries (Variables|Country|Getcountries))
  (Transformation|SetWorldLocation (Variables|Default|Getglobe) (Variables|Default|GetUpperPos) false)
  (bind _returnvalue (Rendering|Material|CreateDynamicMaterialInstance "/Game/Materials/baseColor/TranslucentColor.TranslucentColor" :!class /Script/Engine.KismetMaterialLibrary))
  (Variables|Country|SetCountryMat _returnvalue)
  (Rendering|Material|SetVectorParameterValue (Variables|Country|GetCountryMat) "SolidColor" "(R=1.000000,G=0.061864,B=0.907864,A=1.000000)" :!class /Script/Engine.MaterialInstanceDynamic)
  (for _array_element (Actor|GetComponentsByClass self "/Script/Engine.StaticMeshComponent")
    (bind _asstatic_mesh_component (Utilities|Casting|CastToStaticMeshComponent _array_element))
    (Utilities|Array|Add _countries _asstatic_mesh_component))
  (Utilities|Array|RemoveItem _countries (Variables|Default|Getglobe))
  (for _array_element_2 _countries
    (Rendering|Material|SetMaterial _array_element_2 0 (Variables|Country|GetCountryMat))
    (Rendering|SetVisibility _array_element_2 true false)))

(fn SetSphericalCoord
  (params (sphericalCoords :type Vector%202D%20Structure))
  (bind _rotator (CallFunction|ToRotator sphericalCoords))
  (Transformation|SetWorldRotation (Variables|Default|Getglobe) _rotator false)
  (Variables|Default|SetcurrentRotation _rotator))

(fn SetRotating
  (params (rotationState :type Boolean))
  (Variables|Default|SetisRotating rotationState))

(fn GetRotating
  (return (Variables|Default|GetisRotating)))

(fn ToggleRotating
  (if (Variables|Default|GetisRotating)
    (Variables|Default|SetisRotating false)
    (else
      (Variables|Default|SetisRotating true))))

(fn ResetRotation
  (Transformation|SetWorldRotation (Variables|Default|Getglobe) "0, 0, 0" false))

(fn Goto
  (params (SphericalCoords :type Vector%202D%20Structure) (achievement :type Float%20%28single-precision%29))
  (bind _rotator (CallFunction|ToRotator SphericalCoords))
  (Transformation|SetWorldRotation (Variables|Default|Getglobe) (Math|Rotator|Lerp(Rotator) (Variables|Default|GetcurrentRotation) _rotator achievement) false))

(fn ToRotator
  (params (sphericalCoord :type Vector%202D%20Structure))
  (bind (_x _y) (Math|Vector2D|BreakVector2D sphericalCoord))
  (return (Math|Rotator|CombineRotators (Class|KismetMathLibrary|MakeRot 0.0 _y 0.0) (Class|KismetMathLibrary|MakeRot 0.0 0.0 _x))))

(fn Moveto
  (params (Position :type Vector) (Progress :type Float%20%28single-precision%29))
  (Transformation|SetWorldLocation (Variables|Default|Getglobe) (Math|Vector|Lerp(Vector) (Variables|Default|GetcurrentPosition) Position Progress) false))

(fn GetCountryMesh
  (params (Name :type String))
  (for _array_element (Variables|Country|Getcountries)
    (if (Utilities|Enum|Equal(Enum) (Utilities|Array|Get(acopy) (Utilities|String|ParseIntoArray (Utilities|GetDisplayName _array_element) " ") 1) Name)
      (return _array_element))))

(fn IsCountryValid
  (params (String :type String))
  (LocalVariables|Setfound false)
  (for _array_element (Variables|Country|Getcountries)
    (if (Utilities|Enum|Equal(Enum) (Utilities|Array|Get(acopy) (Utilities|String|ParseIntoArray (Utilities|GetDisplayName _array_element) " ") 1) String)
      (LocalVariables|Setfound true)))
  (return (LocalVariables|Getfound)))