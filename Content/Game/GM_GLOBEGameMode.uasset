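; GM_GLOBEGameMode is the game mode that manages switching between app modes and stores the current language.
; On BeginPlay it spawns a UI_Controller and exposes it through a getter.
; ChangeMode announces the change, ends the old mode, then starts the new one after a half-second delay.
; Each transition messages every registered delegate and calls a matching event.
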(event EventBeginPlay
  (bind _returnvalue (Game|SpawnActorfromClass "/Game/UI/UI_Controller.UI_Controller_C" (Variables|Default|GetDummyTransfrom) false 0))
  (Variables|Default|SetUIControllerInstance _returnvalue))

(event EventOnGameModeStart
  (params (Mode :type GM_MODES%20Enum :default "NewEnumerator0"))
  (for _array_element (Variables|Default|GetDelegates)
    (Class|GMInterface|OnGameModeStart(Message) _array_element Mode))
  (Default|CallOnGameModeStartEvent Mode))

(event EventOnGameModeEnd
  (params (Mode :type GM_MODES%20Enum :default "NewEnumerator0"))
  (for _array_element (Variables|Default|GetDelegates)
    (Class|GMInterface|OnGameModeEnd(Message) _array_element Mode))
  (Default|CallOnGameModeEndEvent Mode))

(event EventOnGameModeChange
  (params (FromMode :type GM_MODES%20Enum :default "NewEnumerator0") (ToMode :type GM_MODES%20Enum :default "NewEnumerator0"))
  (for _array_element (Variables|Default|GetDelegates)
    (Class|GMInterface|OnGameModeChange(Message) _array_element FromMode ToMode))
  (Default|CallOnGameModeChangeEvent FromMode ToMode)
  (CallFunction|OnGameModeEnd FromMode)
  (Utilities|FlowControl|Delay 0.5)
  (CallFunction|OnGameModeStart ToMode))

(fn ConstructionScript)

(fn GetUIController
  (return (Variables|Default|GetUIControllerInstance)))

(fn RegisterGameModeDelegate
  (params (Delegate :type GM%20Interface%20Interface))
  (Utilities|Array|Add (Variables|Default|GetDelegates) Delegate))

(fn ChangeMode
  (params (Mode :type GM_MODES%20Enum :default "NewEnumerator0"))
  (CallFunction|OnGameModeChange (Variables|Default|GetCurrentMode) Mode)
  (Variables|Default|SetCurrentMode Mode))

(fn SetLanguage
  (params (LanguageIdx :type Integer))
  (Variables|General|SetLanguage LanguageIdx))

(fn GetLanguage
  (return (Variables|General|GetLanguage)))