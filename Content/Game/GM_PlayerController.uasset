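; GM_PlayerController sets the player camera's default orthographic width shortly after play begins.
; After a short delay, it computes the viewport aspect ratio from player 0's viewport size and prints the resolution and ratio to screen.
; A threshold branch on that ratio selects the width, but both branches currently assign the same value, so aspect ratio has no effect.
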(event EventBeginPlay
  (bind _returnvalue (Game|GetPlayerController 0))
  (bind (_sizex _sizey) (HUD|GetViewportSize _returnvalue))
  (bind _playercameramanager (Variables|/Script/Engine.PlayerController|GetPlayerCameraManager _returnvalue))
  (bind _returnvalue_2 (Math|Conversions|ToFloat(Integer) _sizey))
  (bind _returnvalue_3 (Math|Conversions|ToFloat(Integer) _sizex))
  (bind _returnvalue_4 (/ _returnvalue_3 _returnvalue_2))
  (Utilities|FlowControl|Delay 1.0)
  (Variables|Default|Setratio _returnvalue_4)
  (Development|PrintString (Utilities|String|Append (Utilities|String|Append (Utilities|String|ToString(Integer) _sizex) " x ") (Utilities|String|ToString(Integer) _sizey)))
  (Development|PrintString (Utilities|String|Append " Ratio: " (Utilities|String|ToString(Float) _returnvalue_4)))
  (if (>= (Variables|Default|Getratio) 0.7)
    (Variables|/Script/Engine.PlayerCameraManager|SetDefaultOrthoWidth _playercameramanager 2.6e+02)
    (else
      (Variables|/Script/Engine.PlayerCameraManager|SetDefaultOrthoWidth _playercameramanager 2.6e+02))))

(fn ConstructionScript)