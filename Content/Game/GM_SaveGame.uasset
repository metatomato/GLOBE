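; GM_SaveGame is, by its name, a save game object that holds star and score records for each achievement category.
; It keeps two parallel arrays, Stars and Scores, indexed by converting the achievement category to an integer.
; Setter functions write with size-to-fit, so the arrays grow as needed, while getters read the entry directly without a bounds check.
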(fn SetStar
  (params (AcheivementType :type GM_ACHEIVEMENTS%20Enum :default "NewEnumerator0") (AcheivementDone :type Boolean))
  (Utilities|Array|SetArrayElem (Variables|Default|GetStars) (Math|Conversions|ToInteger(Byte) AcheivementType) AcheivementDone true))

(fn GetStar
  (params (AcheivementCat :type GM_ACHEIVEMENTS%20Enum :default "NewEnumerator0"))
  (return (Utilities|Array|Get(acopy) (Variables|Default|GetStars) (Math|Conversions|ToInteger(Byte) AcheivementCat))))

(fn SetScore
  (params (AcheivementCat :type GM_ACHEIVEMENTS%20Enum :default "NewEnumerator0") (Score :type Integer))
  (Utilities|Array|SetArrayElem (Variables|Default|GetScores) (Math|Conversions|ToInteger(Byte) AcheivementCat) Score true))

(fn GetScore
  (params (AcheivementCat :type GM_ACHEIVEMENTS%20Enum :default "NewEnumerator0"))
  (return (Utilities|Array|Get(acopy) (Variables|Default|GetScores) (Math|Conversions|ToInteger(Byte) AcheivementCat))))